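; Exploding cow character that detonates when it hits or overlaps an actor whose class is listed in ActorsToExplodeWith.
; On begin play it loops a field animation from a random start position, so instances do not animate in sync.
; Detonation spawns a BP_ExplosionViz sized by ExplosionRange, damages every BP_CannonCharacter within that range (scaled from meters to centimeters), then destroys the cow.
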(event Custom|explode
  ;[1 1 1] Explosion
  (bind _outactors (Actor|GetAllActorsOfClass "/Game/Blueprints/BP_CannonCharacter.BP_CannonCharacter_C"))
  (for _array_element _outactors
    (if (< (Transformation|GetDistanceTo _array_element self) (* (Variables|Default|GetExplosionRange) 1e+02))
      (Class|Damageable|ReceiveDamage _array_element 1)))
  (Actor|DestroyActor))

(event Custom|Spawn%20Explosion
  ;[1 1 1] Explosion
  (bind _returnvalue (Game|SpawnActorfromClass "/Game/Blueprints/BP_ExplosionViz.BP_ExplosionViz_C" (Math|Conversions|ToTransform(Vector) (Transformation|GetActorLocation)) "AlwaysSpawn" 0 0))
  (Variables|/Game/Blueprints/BP_ExplosionViz.BP_ExplosionViz_C|SetExplosionSize _returnvalue (Variables|Default|GetExplosionRange)))

(event EventBeginPlay
  (bind _mesh (Variables|Character|GetMesh))
  ;[1 1 1] Begin Play
  (Components|Animation|PlayAnimation _mesh "/Game/Animations/SK_Cow_Field_Anim.SK_Cow_Field_Anim" true)
  (Components|Animation|SetPosition _mesh (Math|Random|RandomFloatinRange 0.0 2.0) true))

(event Collision|EventHit
  (params (MyComp :type Primitive%20Component%20Object%20Reference) (Other :type Actor%20Object%20Reference) (OtherComp :type Primitive%20Component%20Object%20Reference) (bSelfMoved :type Boolean) (HitLocation :type Vector :default "0, 0, 0") (HitNormal :type Vector :default "0, 0, 0") (NormalImpulse :type Vector :default "0, 0, 0") (Hit :type Hit%20Result%20Structure%20%28by%20ref%29))
  ;[1 1 1] On Hit or Begin Overlap ActorsToExplodeWith -> Explode
  (if (Utilities|Array|ContainsItem (Variables|Default|GetActorsToExplodeWith) (Utilities|GetClass Other))
    (CallFunction|SpawnExplosion)
    (CallFunction|Explode)))

(event Collision|EventActorBeginOverlap
  (params (OtherActor :type Actor%20Object%20Reference))
  ;[1 1 1] On Hit or Begin Overlap ActorsToExplodeWith -> Explode
  (if (Utilities|Array|ContainsItem (Variables|Default|GetActorsToExplodeWith) (Utilities|GetClass OtherActor))
    (CallFunction|SpawnExplosion)
    (CallFunction|Explode)))

(fn ConstructionScript)
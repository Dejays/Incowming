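; Behavior tree node that picks a random wander point for the COW AI on each tick and writes it to the TargetLocation blackboard key.
; It caches the AI_Activator controller, then projects a point 800 units from its pawn at a random horizontal angle.
; A sphere trace checks the path: if the first hit is not an AI_Character, the target falls back to the pawn's current location.
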(event EventTick
  (params (OwnerActor :type Actor%20Object%20Reference) (DeltaSeconds :type Float%20%28single-precision%29))
  (if (!= (Variables|Default|GetAI%20CON%20Ref) 0)
    _
    (else
      (bind _asai_activator (Utilities|Casting|CastToAI_Activator OwnerActor))
      (Variables|Default|SetAI%20CON%20Ref _asai_activator)))
  (Actor|GetAllActorsOfClass "/Game/Blueprints/COW_AI/AI_Character.AI_Character_C")
  (bind _output_get (Variables|Default|SetnewAngle (Math|Random|RandomFloatinRange -1.8e+02 1.8e+02)))
  (bind _output_get_2 (Variables|Default|Settarget (Math|Vector|MakeVector (+ (* 800 (Math|Trig|Cos(Degrees) _output_get)) (.X (Math|Vector|BreakVector (Transformation|GetActorLocation (Pawn|GetControlledPawn (Variables|Default|GetAI%20CON%20Ref)))))) (+ (.Y (Math|Vector|BreakVector (Transformation|GetActorLocation (Pawn|GetControlledPawn (Variables|Default|GetAI%20CON%20Ref))))) (* 800 (Math|Trig|Sin(Degrees) _output_get))) (.Z (Math|Vector|BreakVector (Transformation|GetActorLocation (Pawn|GetControlledPawn (Variables|Default|GetAI%20CON%20Ref))))))))
  (bind _outhits (Collision|MultiSphereTraceForObjects (Transformation|GetActorLocation (Pawn|GetControlledPawn (Variables|Default|GetAI%20CON%20Ref))) (+ _output_get_2 "0, 0,15.000000") 1e+01 (Variables|Default|GetDesiredObjectTypes) false 0 "None"))
  (bind _array_element (Utilities|Array|ForEachLoopwithBreak _outhits :!label _label)
    (:LoopBody
      (if (== (Utilities|GetClass (.HitActor (Collision|BreakHitResult _array_element))) "/Game/Blueprints/COW_AI/AI_Character.AI_Character_C")
        (goto _label Break)
        (else
          (Variables|Default|Settarget (Transformation|GetActorLocation (Pawn|GetControlledPawn (Variables|Default|GetAI%20CON%20Ref))))
          (goto _label Break))))
    (:Completed
      (AI|BehaviorTree|SetBlackboardValueasVector (Variables|Default|GetTargetLocation) (Variables|Default|Gettarget)))))
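; Alien teleport projectile that moves its owning cannon character to the ground beneath it on a key or gamepad press.
; Each tick a downward trace places the sphere, stretches the light beam, and colors both green or red from IsTeleportable, with paired DoOnce gates limiting material updates.
; Triggering re-traces, then either teleports the owner or refunds part of the cooldown and reports failure, destroying the projectile either way.
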(event Custom|ServerCalulateTeleport
  (bind _returnvalue (Transformation|GetActorLocation))
  ;[1 1 1] Manual Teleportation
  (Utilities|FlowControl|Sequence
    (:then_0
      (bind _outhit (Collision|LineTraceByChannel _returnvalue (- _returnvalue "0, 0,100000.000000") "TraceTypeQuery1" false 0 "None"))
      (CallFunction|Teleportation (.ImpactNormal (Collision|BreakHitResult _outhit)) (+ (.Location (Collision|BreakHitResult _outhit)) "0, 0,64.000000")))))

(event Custom|Teleportation
  (params (HitImpact :type Vector) (Future%20Position :type Vector))
  (bind _projectileowner (Variables|Default|GetprojectileOwner))
  ;[1 1 1] Manual Teleportation
  ;;[1 1 1] Call IsTeleportable Function from C++ to check Terrain constraint then Call Succesful or Failed Teleportation Event
  (bind _returnvalue (Class|AlienProjectile|IsTeleportable HitImpact))
  (if _returnvalue
    (bind _asbp_cannon_character (Utilities|Casting|CastToBP_CannonCharacter _projectileowner))
    (Class|CannonCharacter|OnTeleportation _asbp_cannon_character Future%20Position (Transformation|GetActorRotation _projectileowner))
    (else
      (Class|AlienProjectile|OnTeleportationFailed)
      (Class|CannonCharacter|ServerTeleportationFailed _projectileowner (Variables|Default|GetFailureTransform))))
  (Actor|DestroyActor))

(event EventBeginPlay
  (bind _projectilemovement (Variables|Default|GetProjectileMovement))
  ;[1 1 1] Set Initial Speed, Gravity% and Velocity%
  (Variables|Default|SetinitSpeedAlteration 1.0)
  (Variables|/Script/Engine.ProjectileMovementComponent|SetProjectileGravityScale _projectilemovement (Variables|Default|GetGravity%25))
  (Utilities|FlowControl|Delay 0.01)
  (Variables|/Script/Engine.MovementComponent|SetVelocity _projectilemovement (* (Variables|/Script/Engine.MovementComponent|GetVelocity _projectilemovement) (Variables|Default|GetVelocity%25))))

(event EventOnTeleportationFailed
  ;[1 1 1] Event called teleportation failed
  (Class|CooldownTimer|ReduceCooldown (Variables|/Script/Incowming.CooldownSystem|GetAlienCooldown (Variables|/Script/Incowming.CannonCharacter|GetCooldownSystem (Variables|Default|GetprojectileOwner))) (Variables|Default|GetCooldownRefund))
  (Variables|Default|SetFailureTransform (Math|Conversions|ToTransform(Vector) (Transformation|GetWorldLocation (Variables|Default|GetSphere)))))

(event EventTick
  (params (DeltaSeconds :type Float%20%28single-precision%29))
  (bind _returnvalue (Transformation|GetActorLocation))
  (bind _lightbeam_mat (Variables|Default|GetLightBeam%20Mat))
  (bind _spherebeam_mat (Variables|Default|GetSphereBeam%20Mat))
  ;[1 1 1] Visual Update
  (bind _outhit (Collision|LineTraceByChannel _returnvalue (- _returnvalue "0, 0,100000.000000") "TraceTypeQuery1" true 0 "None" true "(R=1.000000,G=0.000000,B=0.000000,A=1.000000)" "(R=0.000000,G=1.000000,B=0.000000,A=1.000000)" 0.0))
  (Transformation|SetWorldLocation (Variables|Default|GetSphere) (.ImpactPoint (Collision|BreakHitResult _outhit)) false false)
  (Transformation|SetWorldScale3D (Variables|Default|GetLightBeam) (Math|Vector|MakeVector 1.5 1.5 (.Z (Math|Vector|BreakVector (/ (- (.TraceStart (Collision|BreakHitResult _outhit)) (.ImpactPoint (Collision|BreakHitResult _outhit))) 5e+01)))))
  ;;[1 1 1] Check if surface is Teleportable, light -> Green, if not light -> Red
  (bind _returnvalue_2 (Class|AlienProjectile|IsTeleportable (.ImpactNormal (Collision|BreakHitResult _outhit))))
  (if _returnvalue_2
    (Utilities|FlowControl|DoOnce false :!label _label
      (:Completed
        (Rendering|Material|SetVectorParameterValue _lightbeam_mat "Color" "(R=0.000000,G=1.000000,B=0.000000,A=1.000000)" :!class /Script/Engine.MaterialInstanceDynamic)
        (Rendering|Material|SetVectorParameterValue _spherebeam_mat "Color" "(R=0.000000,G=1.000000,B=0.000000,A=1.000000)" :!class /Script/Engine.MaterialInstanceDynamic)
        (goto _label_2 Reset)))
    (else
      (Utilities|FlowControl|DoOnce false :!label _label_2
        (:Completed
          (Rendering|Material|SetVectorParameterValue _lightbeam_mat "Color" "(R=1.000000,G=0.000000,B=0.000000,A=1.000000)" :!class /Script/Engine.MaterialInstanceDynamic)
          (Rendering|Material|SetVectorParameterValue _spherebeam_mat "Color" "(R=1.000000,G=0.000000,B=0.000000,A=1.000000)" :!class /Script/Engine.MaterialInstanceDynamic)
          (goto _label Reset))))))

(event Input|KeyboardEvents|P
  (params (Key :type Key%20Structure :default "AnyKey"))
  ;[1 1 1] Manual Teleportation
  (:Pressed
    (CallFunction|ServerCalulateTeleport)))

(event Input|GamepadEvents|GamepadFaceButtonLeft
  (params (Key :type Key%20Structure :default "AnyKey"))
  ;[1 1 1] Manual Teleportation
  (:Pressed
    (CallFunction|ServerCalulateTeleport)))

(fn ConstructionScript
  (bind _returnvalue (Rendering|Material|CreateDynamicMaterialInstance (Variables|Default|GetLightBeam) 0 "/Game/Materials/MasterShaders/M_Alien_LightBeam.M_Alien_LightBeam" :!class /Script/Engine.PrimitiveComponent))
  (Variables|Default|SetLightBeam%20Mat _returnvalue)
  (bind _returnvalue_2 (Rendering|Material|CreateDynamicMaterialInstance (Variables|Default|GetSphere) 0 "/Game/Materials/MasterShaders/M_Alien_LightBeam.M_Alien_LightBeam" :!class /Script/Engine.PrimitiveComponent))
  (Variables|Default|SetSphereBeam%20Mat _returnvalue_2))

(fn CreateBeams)

(fn UpdateBeams)
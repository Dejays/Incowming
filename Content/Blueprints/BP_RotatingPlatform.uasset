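; Platform actor that spins continuously and periodically syncs its rotation across the network.
; Tick applies a local rotation scaled by RotationSpeed and delta time for smooth motion.
; A DoOnce reset by a five-second Delay throttles calls to RunonServer, which passes the Platform component's world rotation to a Multicast event that snaps the actor to it.
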(event Custom|Multicast
  (params (Rotation :type Rotator))
  (Transformation|SetActorRotation Rotation))

(event Custom|Run%20on%20Server
  (CallFunction|Multicast (Transformation|GetWorldRotation (Variables|Default|GetPlatform))))

(event EventTick
  (params (DeltaSeconds :type Float%20%28single-precision%29))
  (Utilities|FlowControl|Sequence
    (:then_0
      (Transformation|AddActorLocalRotation (* (Variables|Default|GetRotationSpeed) DeltaSeconds) false false))
    (:then_1
      (Utilities|FlowControl|DoOnce false :!label _label
        (:Completed
          (CallFunction|RunonServer)
          (Utilities|FlowControl|Delay 5.0)
          (goto _label Reset))))))

(fn ConstructionScript)
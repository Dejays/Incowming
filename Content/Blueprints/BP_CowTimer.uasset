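; Cooldown indicator for a cannon character, showing progress through a dynamic material's fill percentage.
; While Activated, Tick fires a DoOnce that plays one timeline on the fill, then a second scaled to TimeRemaining minus half a second.
; On completion it plays a ting only if the local pawn owns it, calls MoveCDViz on the owner and re-arms.
; A multicast reset deactivates it, calls ReduceCooldown and shows a full green fill.
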(event Custom|PlayTingSound
  (bind _asbp_cannon_character (Utilities|Casting|CastToBP_CannonCharacter (Pawn|GetControlledPawn (Game|GetPlayerController 0))))
  (if (== (Variables|Default|GetCooldownTimerOwner) _asbp_cannon_character)
    (Audio|PlaySound2D "/Game/Audio/Sounds/S_Ting_02.S_Ting_02" 0.1)))

(event Custom|Multicast%20ResetCooldown
  (bind _mid_cow (Variables|Default|GetMID%20Cow))
  ;[1 1 1] Multicast ResetCooldown
  (Variables|Default|SetActivated false)
  (Class|CooldownTimer|ReduceCooldown 1e+02)
  (Rendering|Material|SetVectorParameterValue _mid_cow "ColorFill" "(R=0.000000,G=0.800000,B=0.000000,A=1.000000)" :!class /Script/Engine.MaterialInstanceDynamic)
  (Rendering|Material|SetScalarParameterValue _mid_cow "%" 1.0 :!class /Script/Engine.MaterialInstanceDynamic))

(event EventBeginPlay
  (Transformation|AttachComponentToComponent (Variables|Default|GetLocationSpawn) "None" "SnapToTarget" "SnapToTarget" "SnapToTarget" true)
  (bind _returnvalue (Rendering|Material|CreateDynamicMaterialInstance (Variables|Default|GetViz) 0 "/Game/Materials/Material_Instances/MI_Cooldown_01.MI_Cooldown_01" :!class /Script/Engine.PrimitiveComponent))
  (bind _output_get (Variables|Default|SetMID%20Cow _returnvalue))
  (Rendering|Material|SetVectorParameterValue _output_get "ColorFill" "(R=0.700000,G=0.800000,B=0.800000,A=1.000000)" :!class /Script/Engine.MaterialInstanceDynamic)
  (Rendering|Material|SetScalarParameterValue _output_get "%" 1.0 :!class /Script/Engine.MaterialInstanceDynamic))

(event EventTick
  (params (DeltaSeconds :type Float%20%28single-precision%29))
  (bind _timeremaining (Variables|Default|GetTimeRemaining))
  (bind _returnvalue (- _timeremaining 0.5))
  (if (Variables|Default|GetActivated)
    (Utilities|FlowControl|DoOnce false :!label _label
      (:Completed
        (bind _newtrack_0 (Timeline|Timeline_1 PlayFromStart)
          (:Update
            (Rendering|Material|SetScalarParameterValue (Variables|Default|GetMID%20Cow) "%" _newtrack_0 :!class /Script/Engine.MaterialInstanceDynamic))
          (:Finished
            (bind _newtrack_0_2 (Timeline|Timeline_0 PlayFromStart)
              (:Update
                (if (< _newtrack_0_2 _returnvalue)
                  (Rendering|Material|SetScalarParameterValue (Variables|Default|GetMID%20Cow) "%" (/ _newtrack_0_2 _returnvalue) :!class /Script/Engine.MaterialInstanceDynamic)
                  (else
                    (CallFunction|PlayTingSound)
                    (Variables|Default|SetActivated false)
                    (Utilities|FlowControl|Sequence
                      (:then_0
                        (Timeline|Timeline_0 Stop))
                      (:then_1
                        (bind _asbp_cannon_character (Utilities|Casting|CastToBP_CannonCharacter (Variables|Default|GetCooldownTimerOwner)))
                        (Default|MoveCDViz _asbp_cannon_character)
                        (goto _label Reset)))))))))))))

(event EventResetCooldown
  ;[1 1 1] Multicast ResetCooldown
  (CallFunction|MulticastResetCooldown))

(fn ConstructionScript)
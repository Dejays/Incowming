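; Cow projectile that plays mid-air audio in flight and explodes with sound and particles when it hits something.
; BeginPlay copies the explosion radius into a reference that, per its comment, code uses to query overlapping actors.
; On hit, ShowExplosionRange gates both the radius visualiser and stopping the audio, and the emitter is rotated relative to BeginPLayLocation.
; The Blueprint destroys both actors only when the other is a pig or cow projectile.
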(event EventBeginPlay
  ;[1 1 1] Start cow mid air audio
  (Audio|Components|Audio|Play (Variables|Default|GetCowMidairAudio) 0.0)
  ;[1 1 1] Used in code to query mesh component for overlapping actors
  (Variables|Default|SetExplosionRadiusReference (Variables|Default|GetExplosionRadius)))

(event Collision|EventHit
  (params (MyComp :type Primitive%20Component%20Object%20Reference) (Other :type Actor%20Object%20Reference) (OtherComp :type Primitive%20Component%20Object%20Reference) (bSelfMoved :type Boolean) (HitLocation :type Vector) (HitNormal :type Vector) (NormalImpulse :type Vector :default "0, 0, 0") (Hit :type Hit%20Result%20Structure%20%28by%20ref%29))
  (bind _returnvalue (Utilities|GetClass Other))
  (bind _returnvalue_2 (Transformation|GetActorLocation))
  (bind _beginplaylocation (Variables|Default|GetBeginPLayLocation))
  (bind _returnvalue_3 (Math|Rotator|FindLookatRotation _returnvalue_2 _beginplaylocation))
  (bind (_roll _pitch _yaw) (Math|Rotator|BreakRotator _returnvalue_3))
  (Utilities|FlowControl|Sequence
    (:then_0
      ;[1 1 1] Spawning explosion range visual effect (triggerable)
      (if (Variables|Default|GetShow%20Explosion%20Range)
        (bind _returnvalue_4 (Game|SpawnActorfromClass "/Game/Blueprints/BP_ExplosionViz.BP_ExplosionViz_C" (Math|Conversions|ToTransform(Vector) (Transformation|GetActorLocation)) "Undefined" 0 0))
        (Variables|/Game/Blueprints/BP_ExplosionViz.BP_ExplosionViz_C|SetExplosionSize _returnvalue_4 (Variables|Default|GetExplosion%20Radius))
        ;[1 1 1] Stop cow mid air sound on impact
        (Audio|Components|Audio|Stop (Variables|Default|GetCowMidairAudio))))
    (:then_1
      (Audio|PlaySoundatLocation "/Game/Audio/Sounds/FirstPersonTemplateWeaponFire02.FirstPersonTemplateWeaponFire02" _returnvalue_2 "0, 0, 0" 0.5)
      (Effects|SpawnEmitteratLocation "/Game/particles/ParticleSystems/PS_Explosion_01.PS_Explosion_01" _returnvalue_2 (Math|Rotator|MakeRotator _roll _pitch (+ _yaw 9e+01)))
      ;[1 1 1] On hit, destroy pig and cow projectiles
      (if (== _returnvalue "/Game/Blueprints/BPPigProjectile.BPPigProjectile_C")
        (Actor|DestroyActor Other :!label _label)
        (Actor|DestroyActor)
        (elif (== _returnvalue "BPCowProjectile_C")
          (goto _label))))))

(fn ConstructionScript)
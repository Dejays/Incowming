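; BP_ChunkDestroyer is an actor that hides the chunks of Destructible Components it hits.
; On Hit, it runs an object line trace from the impact point along the hit normal to find a bone name.
; If that name contains "part", it hides that bone, then loops over all socket names, hiding each with physics bodies terminated.
; The overlap event is empty, and some bone-check and debug-print nodes are unreachable.
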(event Collision|EventHit
  (params (MyComp :type Primitive%20Component%20Object%20Reference) (Other :type Actor%20Object%20Reference) (OtherComp :type Primitive%20Component%20Object%20Reference) (bSelfMoved :type Boolean) (HitLocation :type Vector) (HitNormal :type Vector) (NormalImpulse :type Vector :default "0, 0, 0") (Hit :type Hit%20Result%20Structure%20%28by%20ref%29))
  (Utilities|Casting|CastToDestructibleComponent OtherComp)
  (bind _outhit (Collision|LineTraceForObjects HitLocation (+ HitLocation (* HitNormal 5e+02)) (Utilities|Array|MakeArray (Variables|Default|GetObjectType)) false 0 "None"))
  (if (Utilities|String|Contains (Utilities|String|ToString(Name) (.HitBoneName (Collision|BreakHitResult _outhit))) "part")
    (bind _asdestructible_component (Utilities|Casting|CastToDestructibleComponent (.HitComponent (Collision|BreakHitResult _outhit))))
    (Components|SkinnedMesh|HideBonebyName _asdestructible_component (.HitBoneName (Collision|BreakHitResult _outhit)) "PBO_None")
    (for _array_element (Transformation|GetAllSocketNames _asdestructible_component)
      (Components|SkinnedMesh|HideBonebyName _asdestructible_component _array_element "PBO_Term"))))

(event Collision|EventActorBeginOverlap
  (params (OtherActor :type Actor%20Object%20Reference)))

(fn ConstructionScript)
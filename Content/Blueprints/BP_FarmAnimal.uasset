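; BP_FarmAnimal is a wandering cow that explodes when it overlaps a BP_CannonCharacter or registers any hit.
; A looping MoveComponentTo cycle turns it by random yaw offsets and steps it forward on a replicated root, with a randomised animation start.
; Other overlaps reset its heading and reverse the move.
; Exploding damages each cannon character within ExplosionRange, spawns a sized BP_ExplosionViz per victim, then destroys the animal.
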(event Custom|explode
  (bind _outactors (Actor|GetAllActorsOfClass "/Game/Blueprints/BP_CannonCharacter.BP_CannonCharacter_C"))
  (for _array_element _outactors
    (if (< (Transformation|GetDistanceTo _array_element self) (* (Variables|Default|GetExplosionRange) 1e+02))
      (Class|Damageable|ReceiveDamage _array_element 1)
      (CallFunction|SpawnExplosion)))
  (Actor|DestroyActor))

(event Custom|Spawn%20Explosion
  (bind _returnvalue (Game|SpawnActorfromClass "/Game/Blueprints/BP_ExplosionViz.BP_ExplosionViz_C" (Transformation|GetActorTransform) "Undefined" 0 0))
  (Variables|/Game/Blueprints/BP_ExplosionViz.BP_ExplosionViz_C|SetExplosionSize _returnvalue (Variables|Default|GetExplosionRange)))

(event EventBeginPlay
  (bind _returnvalue (VehicleSound|GetRootComponent))
  (bind _returnvalue_2 (Transformation|GetActorLocation))
  (bind _skeletalmesh (Variables|Default|GetSkeletalMesh))
  (bind (_x _y _z) (Math|Vector|BreakVector _returnvalue_2))
  (Class|ActorComponent|SetIsReplicated (Variables|Default|GetDefaultSceneRoot) true)
  (Utilities|FlowControl|Sequence
    (:then_0
      (Components|Animation|PlayAnimation _skeletalmesh "/Game/Animations/SK_Cow_Field_Anim.SK_Cow_Field_Anim" true)
      (Components|Animation|SetPosition _skeletalmesh (Math|Random|RandomFloatinRange 0.0 2.0) true))
    (:then_1
      (if (> (+ (Variables|Default|GetnewAngle) (Math|Random|RandomFloatinRange -5e+01 5e+01)) 1.8e+02) :!label _label
        (Variables|Default|SetnewAngle -179.0)
        (elif (< (+ (Variables|Default|GetnewAngle) (Math|Random|RandomFloatinRange -5e+01 5e+01)) -1.8e+02)
          (Variables|Default|SetnewAngle 179.0)
          (else
            (Variables|Default|SetnewAngle (+ (Variables|Default|GetnewAngle) (Math|Random|RandomFloatinRange -5e+01 5e+01))))))
      (Components|MoveComponentTo _returnvalue _returnvalue_2 (Math|Rotator|MakeRotator 0.0 0.0 (Variables|Default|GetnewAngle)) true true 1.0)
      (Components|MoveComponentTo _returnvalue (Math|Vector|MakeVector (+ (* 50 (Math|Trig|Cos(Degrees) (Variables|Default|GetnewAngle))) _x) (+ _y (* 50 (Math|Trig|Sin(Degrees) (Variables|Default|GetnewAngle)))) _z) (Math|Rotator|MakeRotator 0.0 0.0 (Variables|Default|GetnewAngle)) true true (Math|Random|RandomFloatinRange 1.0 2.0))
      (goto _label))))

(event Collision|EventHit
  (params (MyComp :type Primitive%20Component%20Object%20Reference) (Other :type Actor%20Object%20Reference) (OtherComp :type Primitive%20Component%20Object%20Reference) (bSelfMoved :type Boolean) (HitLocation :type Vector :default "0, 0, 0") (HitNormal :type Vector :default "0, 0, 0") (NormalImpulse :type Vector :default "0, 0, 0") (Hit :type Hit%20Result%20Structure%20%28by%20ref%29))
  (CallFunction|Explode))

(event Collision|EventActorBeginOverlap
  (params (OtherActor :type Actor%20Object%20Reference))
  (bind _returnvalue (VehicleSound|GetRootComponent))
  (bind _returnvalue_2 (Transformation|GetActorLocation))
  (bind (_x _y _z) (Math|Vector|BreakVector _returnvalue_2))
  (if (== (Utilities|GetClass OtherActor) "/Game/Blueprints/BP_CannonCharacter.BP_CannonCharacter_C")
    (CallFunction|Explode)
    (else
      (Variables|Default|SetnewAngle 1.8e+02)
      (Components|MoveComponentTo _returnvalue (Math|Vector|MakeVector (+ (* 50 (Math|Trig|Cos(Degrees) (Variables|Default|GetnewAngle))) _x) (+ _y (* 50 (Math|Trig|Sin(Degrees) (Variables|Default|GetnewAngle)))) _z) (Math|Rotator|MakeRotator 0.0 0.0 (Variables|Default|GetnewAngle)) true true (Math|Random|RandomFloatinRange 1.0 2.0)) ; enters at Return
    )))

(fn ConstructionScript)
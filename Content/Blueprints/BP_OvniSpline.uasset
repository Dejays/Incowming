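; BP_OvniSpline is an actor that flies a spinning Ovni (UFO) along the OvniPath spline, animated only on non-server instances.
; The LocationAlongSpline timeline drives distance and yaw, scaled by MovementSpeed and RotationSpeed.
; BeginTime offsets the construction-script placement and shortens the first cycle.
; A self-looping Delay then restarts the timeline every AnimResetTime.
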(event EventBeginPlay
  (bind _ovni (Variables|Default|GetOvni))
  (if (not (Networking|IsServer))
    (Utilities|FlowControl|Sequence
      (:then_0
        (bind _newtrack_0 (Timeline|Location%20Along%20Spline PlayFromStart)
          (:Update
            (Transformation|SetWorldLocation _ovni (Spline|GetLocationatDistanceAlongSpline (Variables|Default|GetOvniPath) (* _newtrack_0 (Variables|Default|GetMovementSpeed)) "World") false false)
            (Transformation|SetRelativeRotation _ovni (Math|Rotator|MakeRotator 0.0 0.0 (* _newtrack_0 (Variables|Default|GetRotationSpeed))) false false))))
      (:then_1
        (Timeline|Location%20Along%20Spline SetNewTime))
      (:then_2
        (Utilities|FlowControl|Delay (- (Variables|Default|GetAnimResetTime) (Variables|Default|GetBegin%20Time)))
        (Utilities|FlowControl|Sequence
          (:then_0
            (Timeline|Location%20Along%20Spline PlayFromStart))
          (:then_1
            (Utilities|FlowControl|Delay (Variables|Default|GetAnimResetTime) :!label _label)
            (Utilities|FlowControl|Sequence
              (:then_0
                (Timeline|Location%20Along%20Spline PlayFromStart))
              (:then_1
                (goto _label)))))))))

(fn ConstructionScript
  (Transformation|SetWorldLocation (Variables|Default|GetOvni) (Spline|GetLocationatDistanceAlongSpline (Variables|Default|GetOvniPath) (* (Variables|Default|GetBegin%20Time) (Variables|Default|GetMovementSpeed)) "World") false false))
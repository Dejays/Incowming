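; Pig projectile that bounces, with sound and particle feedback on each bounce and on destruction.
; BeginPlay records the spawn location and initial speed, sets the bounce counter, and applies gravity, bounciness, friction and physical material to the movement and sphere components.
; Bounce and destroy events only spawn effects; their triggers and the bounce countdown are not in these graphs.
; Spin and surface-based bounce logic are left unconnected.
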(event Collision|EventActorBeginOverlap
  (params (OtherActor :type Actor%20Object%20Reference)))

(event EventOnProjectileBounce
  (bind _sphere (Variables|Default|GetSphere))
  (bind _returnvalue (Transformation|GetWorldLocation _sphere))
  ;[1 1 1] Play sound at bounce location
  (Audio|PlaySoundatLocation "/Game/Audio/Sounds/S_Pig.S_Pig" _returnvalue)
  ;[1 1 1] Partcile effect at bounce location
  (Effects|SpawnEmitteratLocation "/Game/particles/ParticleSystems/PS_CloudPuff_01.PS_CloudPuff_01" _returnvalue "0.000000,0.000000,90.000000"))

(event EventBeginPlay
  (bind _projectilemovement (Variables|Default|GetProjectileMovement))
  ;[1 0.895 0.1] Initialisation des variable (Pourrait être attribuer dans les valeurs par défauts au lieu de les attribuer au begin play.)
  (Variables|Default|SetBeginPLayLocation (Transformation|GetActorLocation))
  (Variables|Default|SetinitSpeedAlteration (Variables|Default|GetSpeed%25))
  (Variables|/Script/Engine.ProjectileMovementComponent|SetProjectileGravityScale (Variables|Default|GetProjectileMovement) (Variables|Default|GetGravity%25))
  (Variables|Default|SetnbOfBouncesRemaining (Variables|Default|GetNbOfBounces))
  (Variables|/Script/Engine.ProjectileMovementComponent|SetBounciness _projectilemovement (Variables|Default|GetBounciness))
  (Variables|/Script/Engine.ProjectileMovementComponent|SetFriction _projectilemovement (Variables|Default|GetFriction))
  (Class|PrimitiveComponent|SetPhysMaterialOverride (Variables|Default|GetSphere) (Variables|Default|GetPhysical%20Material)))

(event EventOnPigDestroy
  (bind _sphere (Variables|Default|GetSphere))
  (bind _returnvalue (Transformation|GetWorldLocation _sphere))
  ;[1 1 1] Play sound at last bounce/player hit location
  (Audio|PlaySoundatLocation "/Game/Audio/Sounds/FirstPersonTemplateWeaponFire02.FirstPersonTemplateWeaponFire02" _returnvalue "0, 0, 0" 1.0 1.0 0.0 "/Game/Audio/FirstPersonTemplateWeaponFire02Attenuation.FirstPersonTemplateWeaponFire02Attenuation")
  (Effects|SpawnEmitteratLocation "/Game/particles/ParticleSystems/PS_PigBacon_01.PS_PigBacon_01" _returnvalue))

(fn ConstructionScript)
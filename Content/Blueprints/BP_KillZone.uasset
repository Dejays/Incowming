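; BP_KillZone is a volume actor that handles anything that overlaps it.
; An overlapping BP_CannonCharacter is moved to the transform of a randomly chosen PlayerStart in the level, so it respawns without being destroyed.
; Any other actor is destroyed if its exact class is in the ClassesToDestroy list, noted in a comment as Alien, Cow and Pig.
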(event Collision|EventActorBeginOverlap
  (params (OtherActor :type Actor%20Object%20Reference))
  (bind _output_get (Variables|Default|SetOtherActor OtherActor))
  (if (== (Utilities|GetClass _output_get) "/Game/Blueprints/BP_CannonCharacter.BP_CannonCharacter_C")
    ;[1 1 1] If Other Actor == Cannon Character -> Respawn it at Random Player Start
    (bind _outactors (Actor|GetAllActorsOfClass "/Script/Engine.PlayerStart"))
    (Transformation|SetActorTransform (Variables|Default|GetOtherActor) (Transformation|GetActorTransform (Utilities|Array|Get(acopy) _outactors (Math|Random|RandomInteger (Utilities|Array|Length _outactors)))))
    (else
      ;[1 1 1] If Other Actor == Alien || Cow || Pig -> Destroy it
      (if (Utilities|Array|ContainsItem (Variables|Default|GetClassesToDestroy) (Utilities|GetClass (Variables|Default|GetOtherActor)))
        (Actor|DestroyActor (Variables|Default|GetOtherActor))))))

(fn ConstructionScript)
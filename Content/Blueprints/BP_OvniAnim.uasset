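; BP_OvniAnim animates an Ovni (UFO) component with movement and spin from the moment play begins.
; On BeginPlay the OvniAnim_01 timeline plays, with its start time also set there.
; Each update adds a vertical world offset from the ZLoc track, scaled by HeightVar.
; The Rotation track, scaled by RotSpeed, adds yaw in both world and local space, accumulating every tick.
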(event EventBeginPlay
  (bind _rotspeed (Variables|Default|GetRotSpeed))
  (bind _ovni (Variables|Default|GetOvni))
  (Utilities|FlowControl|Sequence
    (:then_0
      (bind (_direction _zloc _rotation) (Timeline|OvniAnim_01 Play)
        (:Update
          (Transformation|AddWorldOffset _ovni (Math|Vector|MakeVector 0.0 0.0 (* _zloc 2.0 (Variables|Default|GetHeightVar))) false false)
          (Transformation|AddWorldRotation _ovni (Math|Rotator|MakeRotator 0.0 0.0 (* _rotation 0.4 _rotspeed)) false false)
          (Transformation|AddLocalRotation (Variables|Default|GetOvni) (Math|Rotator|MakeRotator 0.0 0.0 (* _rotation 0.08 _rotspeed)) false false))))
    (:then_1
      (Timeline|OvniAnim_01 SetNewTime))))

(fn ConstructionScript)
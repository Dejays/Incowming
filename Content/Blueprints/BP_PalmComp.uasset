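; BP_PalmComp is a rotating, destructible mill palm that shatters when hit by animal projectiles and reports its destruction to its Mill.
; Cow projectiles always break it, while pig projectiles do so only with PigVulnerability enabled.
; A hit swaps the static mesh for a destructible one, then applies radial damage near the hit point or at the center of mass.
; The explosion increments the Mill's destroyed-palm count and stops the rotation.
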(event Custom|Explode
  (params (HitLocation :type Vector))
  (bind _impulse_strenght (Variables|Default|GetImpulse%20Strenght))
  (bind _returnvalue (* _impulse_strenght 1e+03))
  ;[1 1 1] Explode the Destructible Mesh, increment Mill's Palms Destroyed and Stop the rotating movement
  (if (Variables|Default|GetExplodeOnHitLocation)
    (Class|DestructibleComponent|ApplyRadiusDamage (Variables|Default|GetDestructibleComp) 5e+02 HitLocation 2e+03 _returnvalue false)
    (else
      (bind _returnvalue_2 (Physics|GetCenterOfMass (Variables|Default|GetDestructibleComp) "None"))
      (Class|DestructibleComponent|ApplyRadiusDamage (Variables|Default|GetDestructibleComp) 5e+02 _returnvalue_2 2e+03 _returnvalue false)))
  (Default|IncrementPalmsDestroyed (Variables|Default|GetMill))
  (Components|Activation|SetActive (Variables|Default|GetRotatingMovement) false false)
  (Variables|Default|SetisRotating false))

(event Custom|SwapToDestructible
  (bind _staticmesh (Variables|Default|GetStaticMesh))
  ;[1 1 1] Swap between static and destructible mesh
  (Development|SetHiddeninGame _staticmesh true false)
  (Collision|SetCollisionEnabled _staticmesh "NoCollision")
  (Class|DestructibleComponent|SetDestructibleMesh (Variables|Default|GetDestructibleComp) "/Game/Environnement/Buildings/SM_BD_Mill_Palm_DM.SM_BD_Mill_Palm_DM"))

(event EventBeginPlay
  ;[1 1 1] Begin Play
  (Variables|/Script/Engine.RotatingMovementComponent|SetRotationRate (Variables|Default|GetRotatingMovement) (Variables|Default|GetRotation%20Speed)))

(event Collision|EventHit
  (params (MyComp :type Primitive%20Component%20Object%20Reference) (Other :type Actor%20Object%20Reference) (OtherComp :type Primitive%20Component%20Object%20Reference) (bSelfMoved :type Boolean) (HitLocation :type Vector) (HitNormal :type Vector) (NormalImpulse :type Vector :default "0, 0, 0") (Hit :type Hit%20Result%20Structure%20%28by%20ref%29))
  (bind _returnvalue (Utilities|GetClass Other))
  (bind _returnvalue_2 (== _returnvalue "/Game/Blueprints/BPCowProjectile.BPCowProjectile_C"))
  ;[1 1 1] Hit with Pig Vulnerabilty and Hit Angle
  (if (Variables|Default|GetPig%20Vulnerability)
    (if (or (== _returnvalue "/Game/Blueprints/BPPigProjectile.BPPigProjectile_C") _returnvalue_2)
      (CallFunction|SwaptoDestructible :!label _label)
      (CallFunction|Explode (+ HitLocation (* HitNormal -5e+02))))
    (elif _returnvalue_2
      (goto _label))))

(fn ConstructionScript)
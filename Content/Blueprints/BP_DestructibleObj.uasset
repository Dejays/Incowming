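; Destructible world object that shatters when hit by cow projectiles, or also by pig projectiles when flagged as pig-vulnerable.
; It shows a static mesh until a one-time swap to a damaged or hidden mesh plus a destructible mesh, also triggered by F.
; Hits then apply radius damage from an offset impact point or center of mass, and spawn an onomatopoeia effect.
; The destructible component is destroyed after a delay.
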(event Custom|Explode
  (params (Hit%20Origin :type Vector))
  (if (Variables|Default|GetExplosionBasedOnHitLocation)
    (Class|DestructibleComponent|ApplyRadiusDamage (Variables|Default|GetDestructibleComp) 5e+02 Hit%20Origin 2e+03 (* (Variables|Default|GetImpulse%20Strenght) 1e+03) false)
    (else
      (bind _returnvalue (Physics|GetCenterOfMass (Variables|Default|GetDestructibleComp) "None"))
      (Class|DestructibleComponent|ApplyRadiusDamage (Variables|Default|GetDestructibleComp) 5e+02 _returnvalue 2e+03 (* (Variables|Default|GetImpulse%20Strenght) 1e+03) false)))
  (Utilities|FlowControl|Delay 1e+01)
  (Components|DestroyComponent (Variables|Default|GetDestructibleComp)))

(event Custom|SwapToDestructible
  (bind _destructiblecomp (Variables|Default|GetDestructibleComp))
  (bind _staticmesh (Variables|Default|GetStaticMesh))
  (if (Variables|Default|GetIsStaticMesh)
    (if (Utilities|IsValid (Variables|Default|GetDamagedMesh))
      (Components|StaticMesh|SetStaticMesh _staticmesh (Variables|Default|GetDamagedMesh))
      (else
        (Development|SetHiddeninGame _staticmesh true false)
        (Collision|SetCollisionEnabled _staticmesh "NoCollision")))
    (Class|DestructibleComponent|SetDestructibleMesh _destructiblecomp (Variables|Default|GetDestructibleMesh))
    (Variables|/Script/Engine.DestructibleComponent|SetLargeChunkThreshold _destructiblecomp 5e+02)
    (Variables|Default|SetIsStaticMesh false)))

(event Collision|EventHit
  (params (MyComp :type Primitive%20Component%20Object%20Reference) (Other :type Actor%20Object%20Reference) (OtherComp :type Primitive%20Component%20Object%20Reference) (bSelfMoved :type Boolean) (HitLocation :type Vector) (HitNormal :type Vector) (NormalImpulse :type Vector :default "0, 0, 0") (Hit :type Hit%20Result%20Structure%20%28by%20ref%29))
  (bind _returnvalue (Utilities|GetClass Other))
  (bind _returnvalue_2 (== _returnvalue "/Game/Blueprints/BPCowProjectile.BPCowProjectile_C"))
  (if (Variables|Default|GetPig%20vulnerable)
    (if (or (== _returnvalue "/Game/Blueprints/BPPigProjectile.BPPigProjectile_C") _returnvalue_2)
      (CallFunction|SwaptoDestructible :!label _label)
      (CallFunction|Explode (+ HitLocation (* HitNormal -5e+02)))
      (bind _returnvalue_3 (Effects|SpawnEmitteratLocation "/Game/particles/ParticleSystems/PS_onomatopoeia_01.PS_onomatopoeia_01" HitLocation))
      (Transformation|SetWorldScale3D _returnvalue_3 "1.500000,1.500000,1.500000"))
    (elif _returnvalue_2
      (goto _label))))

(event Input|KeyboardEvents|F
  (params (Key :type Key%20Structure :default "AnyKey"))
  (:Pressed
    (CallFunction|SwaptoDestructible)))

(fn ConstructionScript
  (Components|StaticMesh|SetStaticMesh (Variables|Default|GetStaticMesh) (Variables|Default|GetUnDamagedMesh)))
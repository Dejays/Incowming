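; BP_ExplosionViz is a short-lived visual actor that shows an animated explosion mesh and then destroys itself.
; On BeginPlay it creates a dynamic material on the mesh and plays a timeline.
; The timeline's Scale curve drives uniform world scale, multiplied by ExplosionSize, and inversely drives the material's Dissolve parameter.
; The actor is destroyed when the timeline finishes.
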(event EventBeginPlay
  (bind _returnvalue (Rendering|Material|CreateDynamicMaterialInstance (Variables|Default|GetExplosionMesh) 0 0 :!class /Script/Engine.PrimitiveComponent))
  (Variables|Default|SetMaterial _returnvalue)
  (bind _scale (Timeline|Timeline_0 Play)
    (:Update
      (Transformation|SetWorldScale3D (Variables|Default|GetExplosionMesh) (Math|Vector|MakeVector (* _scale (Variables|Default|GetExplosionSize)) (* _scale (Variables|Default|GetExplosionSize)) (* _scale (Variables|Default|GetExplosionSize))))
      (Rendering|Material|SetScalarParameterValue (Variables|Default|GetMaterial) "Dissolve" (* (- 1.0 _scale) 2.5) :!class /Script/Engine.MaterialInstanceDynamic))
    (:Finished
      (Actor|DestroyActor))))

(event Collision|EventActorBeginOverlap
  (params (OtherActor :type Actor%20Object%20Reference)))

(fn ConstructionScript)
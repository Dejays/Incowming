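; Destructible palm mill: a rotating base with four child palm actors that stops turning once enough palms are destroyed.
; On BeginPlay it spins the base with a RotatingMovement, then gives each BP_PalmComp child the same rotation rate and a back-reference to the mill.
; IncrementPalmsDestroyed counts losses and, on reaching MaxDestroyedPalms, deactivates the mill's rotation and that of every palm still flagged as rotating.
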(event Custom|Increment%20Palms%20Destroyed
  ;[1 1 1] If the # of Palms Destroyed > Max, stop all rotating movements
  (bind _output_get (Variables|Default|SetPalmsDestroyed (+ (Variables|Default|GetPalmsDestroyed) 1)))
  (if (== _output_get (Variables|Default|GetMax%20Destroyed%20Palms))
    (Components|Activation|SetActive (Variables|Default|GetRotatingMovement) false false)
    (for _array_element (Variables|Default|GetIndependent%20RotatingPalms)
      (if (Variables|/Game/Blueprints/BP_PalmComp.BP_PalmComp_C|GetisRotating _array_element)
        (Components|Activation|SetActive (Variables|/Game/Blueprints/BP_PalmComp.BP_PalmComp_C|GetRotatingMovement _array_element) false false)))))

(event EventBeginPlay
  (bind _rotatingmovement (Variables|Default|GetRotatingMovement))
  (Components|Movement|SetUpdatedComponent _rotatingmovement (Variables|Default|GetBase))
  (Variables|/Script/Engine.RotatingMovementComponent|SetRotationRate _rotatingmovement (Variables|Default|GetRotation%20Speed))
  (CallFunction|InitPalms))

(fn ConstructionScript)

(fn InitPalms
  (bind _asbp_palm_comp (Utilities|Casting|CastToBP_PalmComp (Variables|/Script/Engine.ChildActorComponent|GetChildActor (Variables|Default|GetPalmActor1))))
  (Variables|/Script/Engine.RotatingMovementComponent|SetRotationRate (Variables|/Game/Blueprints/BP_PalmComp.BP_PalmComp_C|GetRotatingMovement _asbp_palm_comp) (Variables|Default|GetRotation%20Speed))
  (Variables|/Game/Blueprints/BP_PalmComp.BP_PalmComp_C|SetMill _asbp_palm_comp self)
  (Utilities|Array|Add (Variables|Default|GetIndependent%20RotatingPalms) _asbp_palm_comp)
  (bind _asbp_palm_comp_2 (Utilities|Casting|CastToBP_PalmComp (Variables|/Script/Engine.ChildActorComponent|GetChildActor (Variables|Default|GetPalmActor2))))
  (Variables|/Script/Engine.RotatingMovementComponent|SetRotationRate (Variables|/Game/Blueprints/BP_PalmComp.BP_PalmComp_C|GetRotatingMovement _asbp_palm_comp_2) (Variables|Default|GetRotation%20Speed))
  (Variables|/Game/Blueprints/BP_PalmComp.BP_PalmComp_C|SetMill _asbp_palm_comp_2 self)
  (Utilities|Array|Add (Variables|Default|GetIndependent%20RotatingPalms) _asbp_palm_comp_2)
  (bind _asbp_palm_comp_3 (Utilities|Casting|CastToBP_PalmComp (Variables|/Script/Engine.ChildActorComponent|GetChildActor (Variables|Default|GetPalmActor3))))
  (Variables|/Script/Engine.RotatingMovementComponent|SetRotationRate (Variables|/Game/Blueprints/BP_PalmComp.BP_PalmComp_C|GetRotatingMovement _asbp_palm_comp_3) (Variables|Default|GetRotation%20Speed))
  (Variables|/Game/Blueprints/BP_PalmComp.BP_PalmComp_C|SetMill _asbp_palm_comp_3 self)
  (Utilities|Array|Add (Variables|Default|GetIndependent%20RotatingPalms) _asbp_palm_comp_3)
  (bind _asbp_palm_comp_4 (Utilities|Casting|CastToBP_PalmComp (Variables|/Script/Engine.ChildActorComponent|GetChildActor (Variables|Default|GetPalmActor4))))
  (Variables|/Script/Engine.RotatingMovementComponent|SetRotationRate (Variables|/Game/Blueprints/BP_PalmComp.BP_PalmComp_C|GetRotatingMovement _asbp_palm_comp_4) (Variables|Default|GetRotation%20Speed))
  (Variables|/Game/Blueprints/BP_PalmComp.BP_PalmComp_C|SetMill _asbp_palm_comp_4 self)
  (Utilities|Array|Add (Variables|Default|GetIndependent%20RotatingPalms) _asbp_palm_comp_4))